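; Third-person shooter player controller that handles Enhanced Input for the controlled BP_Main character.
; BeginPlay adds the IMC_TPS mapping context and caches the pawn as BP_Main.
; Input actions drive control-rotation-relative movement, camera look and jumping.
; Three slot actions set the character's EquippedWeapon and link the matching unarmed, pistol or rifle animation layer to its mesh.
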(event `self.ReceiveBeginPlay`
  (`EnhancedInputSubsystemInterface.AddMappingContext` (pcsubsystem `EnhancedInputLocalPlayerSubsystem` self) "/Game/Input/IMC_TPS.IMC_TPS" 0 (struct))
  (bind _asbp_main (cast `/Game/Blueprint/Character/BP_Main` (`self.K2_GetPawn`)))
  (set `self.BP Main` _asbp_main))

(event `EnhancedInput|/Game/Input/Actions/IA_Move`
  (params (ActionValue :type "Vector2D Structure") (ElapsedSeconds :type "Float (double-precision)") (TriggeredSeconds :type "Float (double-precision)") (InputAction :type "InputAction Object Reference" :default "/Game/Input/Actions/IA_Move.IA_Move"))
  (bind (_returnvalue_roll _returnvalue_pitch _returnvalue_yaw) (`KismetMathLibrary.BreakRotator` (`self.GetControlRotation`)))
  (bind (_returnvalue_roll_2 _returnvalue_pitch_2 _returnvalue_yaw_2) (`KismetMathLibrary.BreakRotator` (`self.GetControlRotation`)))
  ;[0.03616 0.15 0.02585 0.5] Move
  (:`Triggered`
    (`Pawn.AddMovementInput` (`self.BP Main`) (`KismetMathLibrary.GetRightVector` (`KismetMathLibrary.MakeRotator` _returnvalue_roll 0.0 _returnvalue_yaw)) ActionValue_X false)
    (`Pawn.AddMovementInput` (`self.BP Main`) (`KismetMathLibrary.GetForwardVector` (`KismetMathLibrary.MakeRotator` 0.0 0.0 _returnvalue_yaw_2)) ActionValue_Y false)))

(event `EnhancedInput|/Game/Input/Actions/IA_Look`
  (params (ActionValue :type "Vector2D Structure") (ElapsedSeconds :type "Float (double-precision)") (TriggeredSeconds :type "Float (double-precision)") (InputAction :type "InputAction Object Reference" :default "/Game/Input/Actions/IA_Look.IA_Look"))
  (:`Triggered`
    (`self.AddYawInput` ActionValue_X)
    (`self.AddPitchInput` ActionValue_Y)))

(event `EnhancedInput|/Game/Input/Actions/IA_Jump`
  (params (ActionValue :type Boolean) (ElapsedSeconds :type "Float (double-precision)") (TriggeredSeconds :type "Float (double-precision)") (InputAction :type "InputAction Object Reference" :default "/Game/Input/Actions/IA_Jump.IA_Jump"))
  (:`Started`
    (`Character.Jump` (`self.BP Main`))))

(event `EnhancedInput|/Game/Input/Actions/IA_1`
  (params (ActionValue :type Boolean) (ElapsedSeconds :type "Float (double-precision)") (TriggeredSeconds :type "Float (double-precision)") (InputAction :type "InputAction Object Reference" :default "/Game/Input/Actions/IA_1.IA_1"))
  (:`Started`
    (set `/Game/Blueprint/Character/BP_Main.EquippedWeapon` "NewEnumerator0" (`self.BP Main`))
    (`SkeletalMeshComponent.LinkAnimClassLayers` (`Character.Mesh` (`self.BP Main`)) "/Game/Blueprint/Character/ABP/ABP_Unarmed.ABP_Unarmed_C")))

(event `EnhancedInput|/Game/Input/Actions/IA_2`
  (params (ActionValue :type Boolean) (ElapsedSeconds :type "Float (double-precision)") (TriggeredSeconds :type "Float (double-precision)") (InputAction :type "InputAction Object Reference" :default "/Game/Input/Actions/IA_2.IA_2"))
  (:`Triggered`
    (set `/Game/Blueprint/Character/BP_Main.EquippedWeapon` "NewEnumerator1" (`self.BP Main`))
    (`SkeletalMeshComponent.LinkAnimClassLayers` (`Character.Mesh` (`self.BP Main`)) "/Game/Blueprint/Character/ABP/ABP_Pistol.ABP_Pistol_C")))

(event `EnhancedInput|/Game/Input/Actions/IA_3`
  (params (ActionValue :type Boolean) (ElapsedSeconds :type "Float (double-precision)") (TriggeredSeconds :type "Float (double-precision)") (InputAction :type "InputAction Object Reference" :default "/Game/Input/Actions/IA_3.IA_3"))
  (:`Triggered`
    (set `/Game/Blueprint/Character/BP_Main.EquippedWeapon` "NewEnumerator2" (`self.BP Main`))
    (`SkeletalMeshComponent.LinkAnimClassLayers` (`Character.Mesh` (`self.BP Main`)) "/Game/Blueprint/Character/ABP/ABP_Rifle.ABP_Rifle_C")))

(fn `UserConstructionScript`)