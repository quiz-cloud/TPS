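; BP_Main is a character Blueprint that sets up pistol animation and movement tuning, with debug keys for testing.
; On BeginPlay it links the ABP_Pistol anim class layers to the mesh, then SetupStateSetting configures CharacterMovement speed, acceleration and separate braking friction, which ends at zero.
; Debug keys switch global time dilation between normal and slow motion, or play a finger-guns emote montage with a debug print.
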(event Input|KeyboardEvents|DebugKeySubtract
  (params (Key :type Key%20Structure) (ActionValue :type Input%20Action%20Value%20Structure))
  (:Pressed
    (Utilities|Time|SetGlobalTimeDilation 0.1)))

(event Input|KeyboardEvents|DebugKeyAdd
  (params (Key :type Key%20Structure) (ActionValue :type Input%20Action%20Value%20Structure))
  (:Pressed
    (Utilities|Time|SetGlobalTimeDilation 1.0)))

(event EventBeginPlay
  (Components|SkeletalMesh|AnimationBlueprintLinking|LinkAnimClassLayers (Variables|Character|GetMesh) "/Game/Blueprint/Character/ABP/ABP_Pistol.ABP_Pistol_C")
  (CallFunction|SetupStateSetting))

(event Input|KeyboardEvents|DebugKeyTab
  (params (Key :type Key%20Structure :default "None") (ActionValue :type Input%20Action%20Value%20Structure))
  (:Pressed
    (Animation|Montage|PlayMontage 0 "/Game/Blueprint/Animation/MF_Emote_FingerGuns_Montage.MF_Emote_FingerGuns_Montage"
      (:then
        (Development|PrintString "Hello")))))

(fn ConstructionScript)

(fn SetupStateSetting
  (Utilities|FlowControl|Sequence
    (:then_0
      (Variables|/Script/Engine.CharacterMovementComponent|SetMaxWalkSpeed (Variables|Character|GetCharacterMovement) 5e+02))
    (:then_1
      (Variables|/Script/Engine.CharacterMovementComponent|SetMaxAcceleration (Variables|Character|GetCharacterMovement) 1e+03))
    (:then_2
      (Variables|/Script/Engine.CharacterMovementComponent|SetBrakingFriction (Variables|Character|GetCharacterMovement) 1.2e+03))
    (:then_3
      (Variables|/Script/Engine.CharacterMovementComponent|SetBrakingFrictionFactor (Variables|Character|GetCharacterMovement) 0.0))
    (:then_4
      (Variables|/Script/Engine.CharacterMovementComponent|SetBrakingFriction (Variables|Character|GetCharacterMovement) 0.0))
    (:then_5
      (Variables|/Script/Engine.CharacterMovementComponent|SetbUseSeparateBrakingFriction (Variables|Character|GetCharacterMovement) true))))